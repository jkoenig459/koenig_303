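; BP_Turret is an enemy turret that tracks and shoots at the player while they are inside its Range trigger.
; Overlap begin with BP_PlayerChar starts two looping timers by function name, and overlap end clears them.
; FollowPlayer snaps the Pivot toward player 0 at short intervals instead of on Tick.
; FireAtPlayer spawns a BP_TurretProjectile at the ProjectileSpawn transform on a slower interval.
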(event OnComponentBeginOverlap(Range)
  (params (OverlappedComponent :type Primitive%20Component%20Object%20Reference) (OtherActor :type Actor%20Object%20Reference) (OtherComp :type Primitive%20Component%20Object%20Reference) (OtherBodyIndex :type Integer) (bFromSweep :type Boolean) (SweepResult :type Hit%20Result%20Structure%20%28by%20ref%29))
  ;[0.15 0.15 0.15 0.5] start following
  (Utilities|Casting|CastToBP_PlayerChar OtherActor)
  (Utilities|Time|SetTimerbyFunctionName 0 "FollowPlayer" 0.05 true)
  (Utilities|Time|SetTimerbyFunctionName 0 "FireAtPlayer" 0.5 true))

(event OnComponentEndOverlap(Range)
  (params (OverlappedComponent :type Primitive%20Component%20Object%20Reference) (OtherActor :type Actor%20Object%20Reference) (OtherComp :type Primitive%20Component%20Object%20Reference) (OtherBodyIndex :type Integer))
  ;[0.15 0.15 0.15 0.5] stop following
  (Utilities|Casting|CastToBP_PlayerChar OtherActor)
  (Utilities|Time|ClearTimerbyFunctionName 0 "FollowPlayer")
  (Utilities|Time|ClearTimerbyFunctionName 0 "FireAtPlayer"))

(event Custom|FollowPlayer
  ;[0.15 0.15 0.15 0.5] follow player
  (Transformation|SetWorldRotation (Variables|Default|GetPivot) (Math|Rotator|FindLookatRotation (Transformation|GetActorLocation) (Transformation|GetActorLocation (Game|GetPlayerCharacter 0))) false false))

(event Custom|FireAtPlayer
  ;[0.15 0.15 0.15 0.5] fire at player
  (Game|SpawnActorfromClass "/Game/Enemy/Turret/BP_TurretProjectile.BP_TurretProjectile_C" (Transformation|GetWorldTransform (Variables|Default|GetProjectileSpawn)) "Undefined" "MultiplyWithRoot" 0 0))

(fn ConstructionScript)