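; BP_Door is an interactable door that swings open or closed on interaction, but only while it is unlocked.
; A FlipFlop alternates between playing and reversing a Timeline, whose alpha lerps the Arrow component's relative yaw through a quarter turn.
; The Construction Script gives the Cube a dynamic material instance tinted with PickupColor.
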(event EventIntInteract
  (params (PlayerRef :type BP%20Player%20Char%20Object%20Reference))
  (if (Variables|Default|GetisUnlocked)
    (Utilities|FlowControl|FlipFlop
      (:A
        (bind _alpha (Timeline|Timeline Play)
          (:Update
            (Transformation|SetRelativeRotation (Variables|Default|GetArrow) (Math|Rotator|MakeRotator 0.0 0.0 (Math|Float|Lerp 0.0 -9e+01 _alpha)) false false))))
      (:B
        (Timeline|Timeline Reverse)))))

(fn ConstructionScript
  (bind _returnvalue (Rendering|Material|CreateDynamicMaterialInstance (Variables|Default|GetCube) 0 "/Game/Materials/MAT_Color.MAT_Color" "None" :!class /Script/Engine.PrimitiveComponent))
  (bind _output_get (Variables|Default|SetColorDMI _returnvalue))
  (Rendering|Material|SetVectorParameterValue _output_get "Color" (Variables|Default|GetPickupColor) :!class /Script/Engine.MaterialInstanceDynamic))