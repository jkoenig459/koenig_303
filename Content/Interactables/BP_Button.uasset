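; BP_Button is a color-coded pressure button that unlocks its TargetDoor while a matching BP_Physics_Pickup rests in its overlap volume.
; On begin overlap, a pickup with the same PickupColor unlocks the door and plays the Alpha timeline to lower the button.
; Any pickup leaving relocks the door and reverses the timeline, regardless of color.
; The construction script tints the button through a dynamic material instance using PickupColor.
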(event OnComponentBeginOverlap(Overlap)
  (params (OverlappedComponent :type Primitive%20Component%20Object%20Reference) (OtherActor :type Actor%20Object%20Reference) (OtherComp :type Primitive%20Component%20Object%20Reference) (OtherBodyIndex :type Integer) (bFromSweep :type Boolean) (SweepResult :type Hit%20Result%20Structure%20%28by%20ref%29))
  (bind _asbp_physics_pickup (Utilities|Casting|CastToBP_Physics_Pickup OtherActor))
  (if (== (Variables|/Game/Interactables/BP_Physics_Pickup.BP_Physics_Pickup_C|GetPickupColor _asbp_physics_pickup) (Variables|Default|GetPickupColor))
    (Variables|/Game/Interactables/AnimatedInteractables/BP_Door.BP_Door_C|SetisUnlocked (Variables|Default|GettargetDoor) true)
    (bind _progress (Timeline|Alpha Play)
      (:Update
        (Transformation|SetRelativeLocation (Variables|Default|GetButton) (Math|Vector|MakeVector 0.0 0.0 (Math|Float|Lerp 5.0 1.0 _progress)) false false)))))

(event OnComponentEndOverlap(Overlap)
  (params (OverlappedComponent :type Primitive%20Component%20Object%20Reference) (OtherActor :type Actor%20Object%20Reference) (OtherComp :type Primitive%20Component%20Object%20Reference) (OtherBodyIndex :type Integer))
  (Utilities|Casting|CastToBP_Physics_Pickup OtherActor)
  (Variables|/Game/Interactables/AnimatedInteractables/BP_Door.BP_Door_C|SetisUnlocked (Variables|Default|GettargetDoor) false)
  (bind _progress (Timeline|Alpha Reverse)
    (:Update
      (Transformation|SetRelativeLocation (Variables|Default|GetButton) (Math|Vector|MakeVector 0.0 0.0 (Math|Float|Lerp 5.0 1.0 _progress)) false false))))

(fn ConstructionScript
  (bind _returnvalue (Rendering|Material|CreateDynamicMaterialInstance (Variables|Default|GetButton) 0 "/Game/Materials/MAT_Color.MAT_Color" "None" :!class /Script/Engine.PrimitiveComponent))
  (bind _output_get (Variables|Default|SetColorDMI _returnvalue))
  (Rendering|Material|SetVectorParameterValue _output_get "Color" (Variables|Default|GetPickupColor) :!class /Script/Engine.MaterialInstanceDynamic))