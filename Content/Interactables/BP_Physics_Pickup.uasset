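; BP_Physics_Pickup is an interactable physics cube that the player can pick up and drop.
; On interact, if the player is not holding anything, it sets IsHolding, disables physics and collision, and snaps the cube to the player's Arrow1.
; On drop, it detaches and restores collision and physics, leaving IsHolding unchanged.
; The construction script tints each instance with PickupColor through a dynamic material.
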(event EventIntInteract
  (params (PlayerRef :type BP%20Player%20Char%20Object%20Reference))
  (bind _cube (Variables|Default|GetCube))
  (Development|PrintString "E_Pressed")
  (if (not (Variables|/Game/Player/BP_PlayerChar.BP_PlayerChar_C|GetisHolding PlayerRef))
    (Variables|/Game/Player/BP_PlayerChar.BP_PlayerChar_C|SetisHolding PlayerRef true)
    (Physics|SetSimulatePhysics _cube false)
    (Collision|SetCollisionEnabled _cube "NoCollision")
    (Transformation|AttachComponentToComponent (Variables|Default|GetCube) (Variables|/Game/Player/BP_PlayerChar.BP_PlayerChar_C|GetArrow1 PlayerRef) "None" "SnapToTarget" "KeepRelative" "KeepRelative" true)))

(event EventIntDrop
  (params (PlayerRef :type Actor%20Object%20Reference))
  (bind _cube (Variables|Default|GetCube))
  (Development|PrintString "Dropping")
  (Transformation|DetachFromActor "KeepWorld" "KeepWorld" "KeepWorld")
  (Collision|SetCollisionEnabled _cube "QueryAndPhysics")
  (Physics|SetSimulatePhysics _cube true))

(fn ConstructionScript
  (bind _returnvalue (Rendering|Material|CreateDynamicMaterialInstance (Variables|Default|GetCube) 0 "/Game/Materials/MAT_Color.MAT_Color" "None" :!class /Script/Engine.PrimitiveComponent))
  (bind _output_get (Variables|Default|SetColorDMI _returnvalue))
  (Rendering|Material|SetVectorParameterValue _output_get "Color" (Variables|Default|GetPickupColor) :!class /Script/Engine.MaterialInstanceDynamic))